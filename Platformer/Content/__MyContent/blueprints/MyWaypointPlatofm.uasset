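; A moving platform actor with configurable mesh and material that travels along an ordered array of waypoint actors.
; BeginPlay hides the waypoints and starts motion, with PlatformStart called inside the loop, once per waypoint.
; A timeline at Speed play rate lerps between waypoint locations; its event track advances the indices or, with Loop set, jumps back to the first segment.
; Start and Stop functions control the motion.
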(event Custom|Platform%20Start
  (bind _motion_timeline (Variables|Default|GetMotion%20Timeline))
  (CallFunction|SetFirstWaypoint)
  (Components|Timeline|SetPlayRate _motion_timeline (Variables|Default|GetSpeed))
  (Components|Timeline|PlayfromStart _motion_timeline))

(event EventBeginPlay
  (for _array_element (Variables|Default|GetWaypoints)
    (Rendering|SetActorHiddenInGame _array_element true)
    (CallFunction|PlatformStart)))

(event Collision|EventActorBeginOverlap
  (params (OtherActor :type Actor%20Object%20Reference)))

(event EventTick
  (params (DeltaSeconds :type Float%20%28single-precision%29)))

(fn ConstructionScript
  (bind _platform_mesh (Variables|Default|GetPlatform%20Mesh))
  (Components|StaticMesh|SetStaticMesh _platform_mesh (Variables|Default|GetStatic%20Mesh))
  (Rendering|Material|SetMaterial _platform_mesh 0 (Variables|Default|GetMaterial)))

(fn SetPositions
  (bind _waypoints (Variables|Default|GetWaypoints))
  (Variables|Default|SetCuurent%20waypoint%20position (Transformation|GetActorLocation (Utilities|Array|Get(acopy) _waypoints (Variables|Default|GetCurrent%20Waypoint%20Index))))
  (Variables|Default|SetNext%20Wapoint%20Position (Transformation|GetActorLocation (Utilities|Array|Get(acopy) _waypoints (Variables|Default|GetNext%20waypoint%20index)))))

(fn SetFirstWaypoint
  (Variables|Default|SetCurrent%20Waypoint%20Index 0)
  (Variables|Default|SetNext%20waypoint%20index 1)
  (CallFunction|SetPositions))

(fn SetNextWaypoint
  (bind _result (Math|Integer|IncrementInt (Variables|Default|GetCurrent%20Waypoint%20Index))
    (:%20%20
      (Variables|Default|SetNext%20waypoint%20index (+ _result 1))
      (CallFunction|SetPositions))))

(fn PathIsFinished
  (return (== (Variables|Default|GetNext%20waypoint%20index) (- (Utilities|Array|Length (Variables|Default|GetWaypoints)) 1))))

(fn Start
  (CallFunction|PlatformStart))

(fn Stop
  (Audio|Components|Audio|Stop (Variables|Default|GetMotion%20Timeline)))